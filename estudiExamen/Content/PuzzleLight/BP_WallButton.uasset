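; Wall button for a light puzzle that opens a door when three lights show the correct color sequence.
; Overlapping its box with BP_FPSController enables the button's input, and leaving calls DisableInput on the player controller.
; Keys E, T and R each switch one referenced light, then share a check of all three light counters that calls OpenDoor on a match, with debug prints throughout.
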(event OnComponentBeginOverlap(Box)
  (params (OverlappedComponent :type Primitive%20Component%20Object%20Reference) (OtherActor :type Actor%20Object%20Reference) (OtherComp :type Primitive%20Component%20Object%20Reference) (OtherBodyIndex :type Integer) (bFromSweep :type Boolean) (SweepResult :type Hit%20Result%20Structure%20%28by%20ref%29))
  (Utilities|Casting|CastToBP_FPSController OtherActor)
  (Input|EnableInput (Game|GetPlayerController 0))
  (Development|PrintString "character in trigger"))

(event OnComponentEndOverlap(Box)
  (params (OverlappedComponent :type Primitive%20Component%20Object%20Reference) (OtherActor :type Actor%20Object%20Reference) (OtherComp :type Primitive%20Component%20Object%20Reference) (OtherBodyIndex :type Integer))
  (Utilities|Casting|CastToBP_FPSController OtherActor)
  (Input|DisableInput (Game|GetPlayerController 0) 0)
  (Development|PrintString "character out of trigger"))

(event Input|KeyboardEvents|R
  (params (Key :type Key%20Structure :default "None"))
  ;[1 1 1] there's only a button, depending on which key you press, light 0, 1 or 2 will change color
  (:Pressed
    (Default|SwitchLight (Variables|Default|GetlightToChangeColor2))
    (Development|PrintString "R pressed")
    ;[1 1 1] condition for opening door
    (if (Math|Boolean|ANDBoolean (== (Variables|/Game/PuzzleLight/BP_PointLight.BP_PointLight_C|Getcounter (Variables|Default|GetlightToChangeColor1)) 2) (== (Variables|/Game/PuzzleLight/BP_PointLight.BP_PointLight_C|Getcounter (Variables|Default|GetlightToChangeColor2)) 0) (== (Variables|/Game/PuzzleLight/BP_PointLight.BP_PointLight_C|Getcounter (Variables|Default|GetlightToChangeColor0)) 1)) ; if sequence of lights is correct, openDoor
      (Development|PrintString "TRUE, OPEN DOOR" true true "(R=0.000000,G=0.660000,B=1.000000,A=1.000000)" 1e+01)
      (Default|OpenDoor (Variables|Default|GetdoorToOpen))
      (Development|PrintString "call open door" true true "(R=0.000000,G=0.660000,B=1.000000,A=1.000000)" 5.0)
      (else
        (Development|PrintString "false, do not open door")))))

(event Input|KeyboardEvents|T
  (params (Key :type Key%20Structure :default "None"))
  ;[1 1 1] there's only a button, depending on which key you press, light 0, 1 or 2 will change color
  (:Pressed
    (Default|SwitchLight (Variables|Default|GetlightToChangeColor0))
    (Development|PrintString "T pressed")
    ;[1 1 1] condition for opening door
    (if (Math|Boolean|ANDBoolean (== (Variables|/Game/PuzzleLight/BP_PointLight.BP_PointLight_C|Getcounter (Variables|Default|GetlightToChangeColor1)) 2) (== (Variables|/Game/PuzzleLight/BP_PointLight.BP_PointLight_C|Getcounter (Variables|Default|GetlightToChangeColor2)) 0) (== (Variables|/Game/PuzzleLight/BP_PointLight.BP_PointLight_C|Getcounter (Variables|Default|GetlightToChangeColor0)) 1)) ; if sequence of lights is correct, openDoor
      (Development|PrintString "TRUE, OPEN DOOR" true true "(R=0.000000,G=0.660000,B=1.000000,A=1.000000)" 1e+01)
      (Default|OpenDoor (Variables|Default|GetdoorToOpen))
      (Development|PrintString "call open door" true true "(R=0.000000,G=0.660000,B=1.000000,A=1.000000)" 5.0)
      (else
        (Development|PrintString "false, do not open door")))))

(event Input|KeyboardEvents|E
  (params (Key :type Key%20Structure :default "None"))
  ;[1 1 1] there's only a button, depending on which key you press, light 0, 1 or 2 will change color
  (:Pressed
    (Default|SwitchLight (Variables|Default|GetlightToChangeColor1))
    (Development|PrintString "E pressed")
    ;[1 1 1] condition for opening door
    (if (Math|Boolean|ANDBoolean (== (Variables|/Game/PuzzleLight/BP_PointLight.BP_PointLight_C|Getcounter (Variables|Default|GetlightToChangeColor1)) 2) (== (Variables|/Game/PuzzleLight/BP_PointLight.BP_PointLight_C|Getcounter (Variables|Default|GetlightToChangeColor2)) 0) (== (Variables|/Game/PuzzleLight/BP_PointLight.BP_PointLight_C|Getcounter (Variables|Default|GetlightToChangeColor0)) 1)) ; if sequence of lights is correct, openDoor
      (Development|PrintString "TRUE, OPEN DOOR" true true "(R=0.000000,G=0.660000,B=1.000000,A=1.000000)" 1e+01)
      (Default|OpenDoor (Variables|Default|GetdoorToOpen))
      (Development|PrintString "call open door" true true "(R=0.000000,G=0.660000,B=1.000000,A=1.000000)" 5.0)
      (else
        (Development|PrintString "false, do not open door")))))

(fn ConstructionScript)