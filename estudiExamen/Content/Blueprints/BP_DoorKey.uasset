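; BP_DoorKey is a key-locked door that swings open when a BP_FPSController holding at least one key enters its Box trigger.
; Begin overlap checks the Keys count without decrementing it, then enables input and rotates the actor's root in place via MoveComponentTo, behind a DoOnce that is reset afterwards.
; End overlap disables input and rotates the root back to zero rotation, with no key check.
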(event OnComponentBeginOverlap(Box)
  (params (OverlappedComponent :type Primitive%20Component%20Object%20Reference) (OtherActor :type Actor%20Object%20Reference) (OtherComp :type Primitive%20Component%20Object%20Reference) (OtherBodyIndex :type Integer) (bFromSweep :type Boolean) (SweepResult :type Hit%20Result%20Structure%20%28by%20ref%29))
  (bind _defaultsceneroot (Variables|Default|GetDefaultSceneRoot))
  (bind _returnvalue (Components|GetOwner _defaultsceneroot))
  ;[1 1 1] Key Door opens
  (bind _asbp_fpscontroller (Utilities|Casting|CastToBP_FPSController OtherActor))
  (if (>= (Variables|/Game/Blueprints/BP_FPSController.BP_FPSController_C|GetKeys _asbp_fpscontroller) 1)
    (Utilities|FlowControl|DoOnce false :!label _label
      (:Completed
        (Input|EnableInput 0)
        (Components|MoveComponentTo (Variables|/Script/Engine.Actor|GetRootComponent _returnvalue) (Transformation|GetActorLocation _returnvalue) "0,90.000000, 0" false false 1.0 false)
        (goto _label Reset)))))

(event OnComponentEndOverlap(Box)
  (params (OverlappedComponent :type Primitive%20Component%20Object%20Reference) (OtherActor :type Actor%20Object%20Reference) (OtherComp :type Primitive%20Component%20Object%20Reference) (OtherBodyIndex :type Integer))
  (bind _defaultsceneroot (Variables|Default|GetDefaultSceneRoot))
  (bind _returnvalue (Components|GetOwner _defaultsceneroot))
  ;[1 1 1] Key Door closes
  (Utilities|Casting|CastToBP_FPSController OtherActor)
  (Input|DisableInput 0)
  (Components|MoveComponentTo (Variables|/Script/Engine.Actor|GetRootComponent _returnvalue) (Transformation|GetActorLocation _returnvalue) "0, 0, 0" false false 1.0 false))

(fn ConstructionScript)