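; BP_DoorAutomatic is a door that swings open when a BP_FPSController actor enters its Box trigger and closes when it leaves.
; Overlap events enable or disable input and use MoveComponentTo on the root component to rotate it over time, keeping the actor's current location.
; Opening passes through a DoOnce that is never reset, so it runs only on the first entry, while closing runs on every exit.
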(event OnComponentBeginOverlap(Box)
  (params (OverlappedComponent :type Primitive%20Component%20Object%20Reference) (OtherActor :type Actor%20Object%20Reference) (OtherComp :type Primitive%20Component%20Object%20Reference) (OtherBodyIndex :type Integer) (bFromSweep :type Boolean) (SweepResult :type Hit%20Result%20Structure%20%28by%20ref%29))
  (bind _defaultsceneroot (Variables|Default|GetDefaultSceneRoot))
  (bind _returnvalue (Components|GetOwner _defaultsceneroot))
  ;[1 1 1] Open door
  (Utilities|Casting|CastToBP_FPSController OtherActor)
  (Input|EnableInput 0)
  (Utilities|FlowControl|DoOnce false
    (:Completed
      (Components|MoveComponentTo (Variables|/Script/Engine.Actor|GetRootComponent _returnvalue) (Transformation|GetActorLocation _returnvalue) "0,90.000000, 0" false false 1.0 false))))

(event OnComponentEndOverlap(Box)
  (params (OverlappedComponent :type Primitive%20Component%20Object%20Reference) (OtherActor :type Actor%20Object%20Reference) (OtherComp :type Primitive%20Component%20Object%20Reference) (OtherBodyIndex :type Integer))
  (bind _defaultsceneroot (Variables|Default|GetDefaultSceneRoot))
  (bind _returnvalue (Components|GetOwner _defaultsceneroot))
  ;[1 1 1] Close door
  (Utilities|Casting|CastToBP_FPSController OtherActor)
  (Input|DisableInput 0)
  (Components|MoveComponentTo (Variables|/Script/Engine.Actor|GetRootComponent _returnvalue) (Transformation|GetActorLocation _returnvalue) "0, 0, 0" false false 1.0 false))

(fn ConstructionScript)